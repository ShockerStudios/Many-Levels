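; BP_GraveStoneDoor is a gate that opens once it has received enough tokens.
; Each TokenSent event runs TokenRecieved, which counts tokens and calls GateUnlocked on the one that reaches MaxTokens.
; GateUnlocked plays the DoorActivation timeline to drive the GateDoor's relative Z location.
; SwitchActivated counts pressure switches against a required total, but reaching it triggers nothing.
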(event Custom|SwitchActivated
  (Math|Integer|IncrementInt (Variables|Default|GetPressureSwitchesActive)
    (:%20%20
      (if (>= (Variables|Default|GetPressureSwitchesActive) (Variables|Default|GetPressureSwitchesNeeded))
        _))))

(event Custom|TokenSent
  (CallFunction|TokenRecieved))

(event Custom|GateUnlocked
  (bind _door_position (Timeline|Door%20Activation Play)
    (:Update
      (Transformation|SetRelativeLocation (Variables|Default|GetGateDoor) (Math|Vector|MakeVector 0.0 0.0 _door_position) false false))))

(event EventBeginPlay)

(event Collision|EventActorBeginOverlap
  (params (OtherActor :type Actor%20Object%20Reference)))

(event EventTick
  (params (DeltaSeconds :type Float%20%28single-precision%29)))

(fn ConstructionScript)

(fn TokenRecieved
  (if (>= (Variables|Default|GetCurrentTokens) (- (Variables|Default|GetMaxTokens) 1))
    (CallFunction|GateUnlocked)
    (else
      (bind _result (Math|Integer|IncrementInt (Variables|Default|GetCurrentTokens))
        (:%20%20
          (Variables|Default|SetCurrentTokens _result))))))