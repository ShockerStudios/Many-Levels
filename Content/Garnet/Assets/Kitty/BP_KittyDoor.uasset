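; BP_KittyDoor is a gate door driven by how many pressure switches are active.
; SwitchActivated and SwitchDeactivated adjust a counter, then play the DoorActivation timeline if it meets the required count, or reverse it otherwise.
; Each timeline update sets the door's relative Z to its current world Z plus a fixed offset, rather than interpolating between closed and open positions.
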(event Custom|SwitchActivated
  (Math|Integer|IncrementInt (Variables|Default|GetPressureSwitchesActive)
    (:%20%20
      (if (>= (Variables|Default|GetPressureSwitchesActive) (Variables|Default|GetPressureSwitchesNeeded))
        (Timeline|Door%20Activation Play
          (:Update
            (Transformation|SetRelativeLocation (Variables|Default|GetGateDoor) (Math|Vector|MakeVector 0.0 0.0 (.z (+ (Transformation|GetWorldLocation (Variables|Default|GetGateDoor)) (Math|Vector|MakeVector 0.0 0.0 1e+02)))) false false)))
        (else
          (Timeline|Door%20Activation Reverse))))))

(event Custom|SwitchDeactivated
  (Math|Integer|DecrementInt (Variables|Default|GetPressureSwitchesActive)
    (:%20%20
      (if (>= (Variables|Default|GetPressureSwitchesActive) (Variables|Default|GetPressureSwitchesNeeded))
        (Timeline|Door%20Activation Play
          (:Update
            (Transformation|SetRelativeLocation (Variables|Default|GetGateDoor) (Math|Vector|MakeVector 0.0 0.0 (.z (+ (Transformation|GetWorldLocation (Variables|Default|GetGateDoor)) (Math|Vector|MakeVector 0.0 0.0 1e+02)))) false false)))
        (else
          (Timeline|Door%20Activation Reverse))))))

(event EventBeginPlay)

(event Collision|EventActorBeginOverlap
  (params (OtherActor :type Actor%20Object%20Reference)))

(event EventTick
  (params (DeltaSeconds :type Float%20%28single-precision%29)))

(fn ConstructionScript)