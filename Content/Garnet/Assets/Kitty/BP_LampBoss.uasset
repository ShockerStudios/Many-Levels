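; BP_LampBoss is a lamp actor that lights up once enough pressure switches are active.
; Each SwitchActivated call increments a counter and compares it with the required switch count.
; On reaching that count, it makes its four point lights visible; the graph has no logic to decrement the counter or hide them again.
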(event Custom|SwitchActivated
  (Math|Integer|IncrementInt (Variables|Default|GetPressureSwitchesActive)
    (:%20%20
      (if (>= (Variables|Default|GetPressureSwitchesActive) (Variables|Default|GetPressureSwitchesNeeded))
        (Rendering|SetVisibility (Variables|Default|GetPointLight3) true false)))))

(event EventBeginPlay)

(event Collision|EventActorBeginOverlap
  (params (OtherActor :type Actor%20Object%20Reference)))

(event EventTick
  (params (DeltaSeconds :type Float%20%28single-precision%29)))

(fn ConstructionScript)