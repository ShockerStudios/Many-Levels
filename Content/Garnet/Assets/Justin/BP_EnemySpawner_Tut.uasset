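; BP_EnemySpawner_Tut is a tutorial enemy spawner that the player can destroy by touch, counting toward BP_Gate2.
; From BeginPlay it loops on a SpawnTimer delay, spawning BP_AI_Enemies at its Sphere's transform whenever Activated is true.
; When BP_Devvy overlaps the Capsule, it decrements Tut2Check on the BP_Gate2 found by class lookup, then destroys itself.
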(event OnComponentBeginOverlap(Capsule)
  (params (OverlappedComponent :type Primitive%20Component%20Object%20Reference) (OtherActor :type Actor%20Object%20Reference) (OtherComp :type Primitive%20Component%20Object%20Reference) (OtherBodyIndex :type Integer) (bFromSweep :type Boolean) (SweepResult :type Hit%20Result%20Structure%20%28by%20ref%29))
  (Utilities|Casting|CastToBP_Devvy OtherActor)
  (Utilities|FlowControl|Sequence
    (:then_0
      (bind _returnvalue (Actor|GetActorOfClass "/Game/Garnet/Assets/Justin/BP_Gate2.BP_Gate2_C"))
      (bind _asbp_gate_2 (Utilities|Casting|CastToBP_Gate2 _returnvalue))
      (Variables|/Game/Garnet/Assets/Justin/BP_Gate2.BP_Gate2_C|SetTut2_Check _asbp_gate_2 (- (Variables|/Game/Garnet/Assets/Justin/BP_Gate2.BP_Gate2_C|GetTut2_Check _asbp_gate_2) 1)))
    (:then_1
      (Actor|DestroyActor self))))

(event EventBeginPlay
  (Utilities|FlowControl|Delay (Variables|Default|GetSpawnTimer) :!label _label)
  (if (Variables|Default|GetActivated)
    (Game|SpawnActorfromClass "/Game/Garnet/Assets/Justin/BP_AI_Enemies.BP_AI_Enemies_C" (Transformation|GetWorldTransform (Variables|Default|GetSphere)) "Undefined" 0 0)
    (goto _label)
    (else
      (goto _label))))

(fn ConstructionScript)