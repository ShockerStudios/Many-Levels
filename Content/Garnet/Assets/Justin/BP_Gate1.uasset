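; BP_Gate1 is a gate that slides its static mesh vertically, apparently tied to tutorial progress through TutCheck.
; On BeginPlay, MoveComponentTo raises the mesh over a few seconds.
; Tick polls TutCheck, which is not set in these graphs, and while it is zero requests an equal downward move from the mesh's current position, with no one-shot guard.
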(event EventBeginPlay
  (bind _staticmeshcomponent (Variables|Debug|GetStaticMeshComponent))
  (bind _relativelocation (Variables|/Script/Engine.SceneComponent|GetRelativeLocation _staticmeshcomponent))
  (Components|MoveComponentTo _staticmeshcomponent (Math|Vector|MakeVector (.x _relativelocation) (.y _relativelocation) (+ (.z _relativelocation) 2.5e+02)) (Variables|/Script/Engine.SceneComponent|GetRelativeRotation _staticmeshcomponent) false false 5.0 false))

(event EventTick
  (params (DeltaSeconds :type Float%20%28single-precision%29))
  (bind _staticmeshcomponent (Variables|Debug|GetStaticMeshComponent))
  (bind _relativelocation (Variables|/Script/Engine.SceneComponent|GetRelativeLocation _staticmeshcomponent))
  (if (== (Variables|Default|GetTut_Check) 0)
    (Components|MoveComponentTo _staticmeshcomponent (Math|Vector|MakeVector (.x _relativelocation) (.y _relativelocation) (+ (.z _relativelocation) -2.5e+02)) (Variables|/Script/Engine.SceneComponent|GetRelativeRotation _staticmeshcomponent) false false 5.0 false)))

(fn ConstructionScript)