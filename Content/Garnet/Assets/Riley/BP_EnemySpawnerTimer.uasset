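; Enemy spawner that periodically spawns BP_AI_EnemiesTimer at its Sphere component while activated by the player (BP_Devvy).
; BeginPlay runs an endless Delay loop on SpawnTimer, spawning only while Activated is set.
; Box overlap sets Activated, clears it after a fixed delay, and spawns one enemy immediately on the first entry.
; Capsule overlap with BP_Devvy destroys the spawner.
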(event OnComponentBeginOverlap(Box)
  (params (OverlappedComponent :type Primitive%20Component%20Object%20Reference) (OtherActor :type Actor%20Object%20Reference) (OtherComp :type Primitive%20Component%20Object%20Reference) (OtherBodyIndex :type Integer) (bFromSweep :type Boolean) (SweepResult :type Hit%20Result%20Structure%20%28by%20ref%29))
  (Utilities|Casting|CastToBP_Devvy OtherActor)
  (if (Variables|Default|GetFirstPlayerEnter)
    _
    (else
      (Variables|Default|SetFirstPlayerEnter true)
      (Game|SpawnActorfromClass "/Game/Garnet/Assets/Riley/BP_AI_EnemiesTimer.BP_AI_EnemiesTimer_C" (Transformation|GetWorldTransform (Variables|Default|GetSphere)) "Undefined" 0 0)))
  (Variables|Default|SetActivated true)
  (Utilities|FlowControl|Delay 7.0)
  (Variables|Default|SetActivated false))

(event OnComponentBeginOverlap(Capsule)
  (params (OverlappedComponent :type Primitive%20Component%20Object%20Reference) (OtherActor :type Actor%20Object%20Reference) (OtherComp :type Primitive%20Component%20Object%20Reference) (OtherBodyIndex :type Integer) (bFromSweep :type Boolean) (SweepResult :type Hit%20Result%20Structure%20%28by%20ref%29))
  (Utilities|Casting|CastToBP_Devvy OtherActor)
  (Actor|DestroyActor self))

(event EventBeginPlay
  (Utilities|FlowControl|Delay (Variables|Default|GetSpawnTimer) :!label _label)
  (if (Variables|Default|GetActivated)
    (Game|SpawnActorfromClass "/Game/Garnet/Assets/Riley/BP_AI_EnemiesTimer.BP_AI_EnemiesTimer_C" (Transformation|GetWorldTransform (Variables|Default|GetSphere)) "Undefined" 0 0)
    (goto _label)
    (else
      (goto _label))))

(fn ConstructionScript)