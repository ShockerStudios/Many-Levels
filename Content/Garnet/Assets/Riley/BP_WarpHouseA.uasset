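; BP_WarpHouseA is a locked-door warp actor that opens once its ObtainKey event sets KeyIsGotten.
; While locked, the Box overlap prints a hint to find an unlock button; once unlocked, Tick hides both castle doors and repositions Warpoint every frame.
; Warpoint then moves overlapping actors to Arrow1's world transform, zeroing the player's velocity.
; The construction script places a separate Arrow from TeleportLocation, which the warp does not use.
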(event OnComponentBeginOverlap(Box)
  (params (OverlappedComponent :type Primitive%20Component%20Object%20Reference) (OtherActor :type Actor%20Object%20Reference) (OtherComp :type Primitive%20Component%20Object%20Reference) (OtherBodyIndex :type Integer) (bFromSweep :type Boolean) (SweepResult :type Hit%20Result%20Structure%20%28by%20ref%29))
  (if (not (Variables|Default|GetKeyIsGotten))
    (Development|PrintString "Hmm doors lock I should look for a button to unlock it...")))

(event OnComponentBeginOverlap(Warpoint)
  (params (OverlappedComponent :type Primitive%20Component%20Object%20Reference) (OtherActor :type Actor%20Object%20Reference) (OtherComp :type Primitive%20Component%20Object%20Reference) (OtherBodyIndex :type Integer) (bFromSweep :type Boolean) (SweepResult :type Hit%20Result%20Structure%20%28by%20ref%29))
  (bind _returnvalue (Game|GetPlayerCharacter 0))
  (bind _arrow1 (Variables|Default|GetArrow1))
  (bind _returnvalue_2 (Transformation|GetWorldTransform _arrow1))
  (if (Variables|Default|GetKeyIsGotten)
    (Transformation|SetWorldTransform (Variables|/Script/Engine.Actor|GetRootComponent OtherActor) (Math|Transform|MakeTransform (.location _returnvalue_2) (.rotation _returnvalue_2) "1.000000,1.000000,1.000000") false false)
    (if (== OtherActor _returnvalue)
      (Variables|/Script/Engine.MovementComponent|SetVelocity (Variables|/Script/Engine.Character|GetCharacterMovement _returnvalue) "0, 0, 0"))))

(event Custom|ObtainKey
  (Variables|Default|SetKeyIsGotten true))

(event EventBeginPlay)

(event Collision|EventActorBeginOverlap
  (params (OtherActor :type Actor%20Object%20Reference)))

(event EventTick
  (params (DeltaSeconds :type Float%20%28single-precision%29))
  (if (Variables|Default|GetKeyIsGotten)
    (Rendering|SetVisibility (Variables|Default|GetSM_Bld_Castle_Door_R) false false)
    (Rendering|SetVisibility (Variables|Default|GetSM_Bld_Castle_Door_L) false false)
    (Transformation|SetRelativeLocation (Variables|Default|GetWarpoint) "0.000000,14.285715,66.666664" false false)))

(fn ConstructionScript
  (Transformation|SetRelativeTransform (Variables|Default|GetArrow) (Variables|Default|Getteleport%20location) false false))