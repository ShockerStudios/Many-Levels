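; Lamp actor with a point light that plays a quiet buzz when BP_Devvy enters its sphere.
; On overlap it fetches the LampBuzzingManager nearest the world origin and proceeds only if PlayingLampBuzzing is true.
; It then calls NoBuzz, plays the sound at the light and calls PlayBuzz after a delay, using the manager as a shared gate.
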(event OnComponentBeginOverlap(Sphere)
  (params (OverlappedComponent :type Primitive%20Component%20Object%20Reference) (OtherActor :type Actor%20Object%20Reference) (OtherComp :type Primitive%20Component%20Object%20Reference) (OtherBodyIndex :type Integer) (bFromSweep :type Boolean) (SweepResult :type Hit%20Result%20Structure%20%28by%20ref%29))
  (Utilities|Casting|CastToBP_Devvy OtherActor)
  (bind _outactors (Actor|GetAllActorsOfClass "/Game/Garnet/Assets/Riley/lampBuzzingManager.lampBuzzingManager_C"))
  (bind _aslamp_buzzing_manager (Utilities|Casting|CastTolampBuzzingManager (.ReturnValue (Actor|FindNearestActor "0, 0, 0" _outactors))))
  (Variables|Default|SetAs%20Lamp%20Buzzing%20Manager _aslamp_buzzing_manager)
  (if (Variables|/Game/Garnet/Assets/Riley/lampBuzzingManager.lampBuzzingManager_C|GetPlaying%20Lamp%20Buzzing (Variables|Default|GetAs%20Lamp%20Buzzing%20Manager))
    (Default|NoBuzz (Variables|Default|GetAs%20Lamp%20Buzzing%20Manager))
    (Audio|PlaySoundatLocation "/Game/Garnet/Assets/Riley/Sounds/LampBuzz_CUE.LampBuzz_CUE" (Transformation|GetWorldLocation (Variables|Default|GetPointLight)) "0, 0, 0" 0.2 1.0 0.0 0 0 0 0)
    (Utilities|FlowControl|Delay 6.0)
    (Default|PlayBuzz (Variables|Default|GetAs%20Lamp%20Buzzing%20Manager))))

(event EventBeginPlay)

(event Collision|EventActorBeginOverlap
  (params (OtherActor :type Actor%20Object%20Reference)))

(event EventTick
  (params (DeltaSeconds :type Float%20%28single-precision%29)))

(fn ConstructionScript)