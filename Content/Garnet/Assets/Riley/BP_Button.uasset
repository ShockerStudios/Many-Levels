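; BP_Button is a one-shot trigger button that activates when a BP_Devvy or BP_AI_Minions actor overlaps its Collider.
; A Sequence tries both casts, and either success runs shared logic that swaps the unused mesh for the used one and sets IsButtonActive.
; It prints the flag and destroys the Collider so it cannot retrigger, leaving no path to reset it.
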(event OnComponentBeginOverlap(Collider)
  (params (OverlappedComponent :type Primitive%20Component%20Object%20Reference) (OtherActor :type Actor%20Object%20Reference) (OtherComp :type Primitive%20Component%20Object%20Reference) (OtherBodyIndex :type Integer) (bFromSweep :type Boolean) (SweepResult :type Hit%20Result%20Structure%20%28by%20ref%29))
  (Utilities|FlowControl|Sequence
    (:then_0
      (Utilities|Casting|CastToBP_Devvy OtherActor))
    (:then_1
      (Utilities|Casting|CastToBP_AI_Minions OtherActor)))
  (Rendering|SetVisibility (Variables|Default|GetButtonUnused) false false)
  (Rendering|SetVisibility (Variables|Default|GetButtonUsed) true false)
  (bind _output_get (Variables|Default|SetIsButtonActive? true))
  (Development|PrintString (Utilities|String|ToString(Boolean) _output_get))
  (Components|DestroyComponent (Variables|Default|GetCollider)))

(event EventBeginPlay)

(event Collision|EventActorBeginOverlap
  (params (OtherActor :type Actor%20Object%20Reference)))

(event EventTick
  (params (DeltaSeconds :type Float%20%28single-precision%29)))

(fn ConstructionScript)