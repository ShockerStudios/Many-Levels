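; BP_Button_Child is a one-shot overlap button that, judging by its name, derives from a parent button Blueprint.
; When BP_Devvy enters the Collider, it swaps the unused mesh for the used one and marks the button active.
; It then destroys the Collider so it cannot retrigger, finds a Gate actor by class lookup and calls GetKey on it.
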(event OnComponentBeginOverlap(Collider)
  (params (OverlappedComponent :type Primitive%20Component%20Object%20Reference) (OtherActor :type Actor%20Object%20Reference) (OtherComp :type Primitive%20Component%20Object%20Reference) (OtherBodyIndex :type Integer) (bFromSweep :type Boolean) (SweepResult :type Hit%20Result%20Structure%20%28by%20ref%29))
  (Utilities|Casting|CastToBP_Devvy OtherActor)
  (Rendering|SetVisibility (Variables|Default|GetButtonUnused) false false)
  (Rendering|SetVisibility (Variables|Default|GetButtonUsed) true false)
  (bind _output_get (Variables|Default|SetIsButtonActive? true))
  (Components|DestroyComponent (Variables|Default|GetCollider))
  (bind _returnvalue (Actor|GetActorOfClass "/Game/Garnet/Assets/Riley/Gate.Gate_C"))
  (bind _asgate (Utilities|Casting|CastToGate _returnvalue))
  (Default|GetKey _asgate))

(event EventBeginPlay
  (|CallParentFunction) ; This node is disabled and will not be called.\nDrag off pins to build functionality.
)

(event EventTick
  (params (DeltaSeconds :type Float%20%28single-precision%29))
  (|CallParentFunction DeltaSeconds) ; This node is disabled and will not be called.\nDrag off pins to build functionality.
)

(fn ConstructionScript
  (|CallParentFunction))