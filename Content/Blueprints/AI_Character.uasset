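; AI character that carries out three commands: follow a target, wait in place, or move to a location.
; Each command event records itself in ActiveCommand, then either issues an AIMoveTo or stops active movement.
; Following is a latent loop that, one second after each move succeeds or fails, re-issues the move if FollowMe is still the active command.
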(event Custom|Follow%20Me
  (params (Follow%20Target :type Actor%20Object%20Reference))
  (Variables|Default|SetActive%20Command "NewEnumerator0")
  (AI|AIMoveTo self "0, 0, 0" Follow%20Target 1e+01 false :!label _label
    (:OnSuccess
      _)
    (:OnFail
      _))
  (Utilities|FlowControl|Delay 1.0)
  (switch Utilities|FlowControl|Switch|SwitchonAI_Commands (Variables|Default|GetActive%20Command)
    (:NewEnumerator0
      (goto _label))))

(event Custom|Wait
  (Variables|Default|SetActive%20Command "NewEnumerator1")
  (Class|NavMovementComponent|StopActiveMovement (Variables|Character|GetCharacterMovement)))

(event Custom|Move%20There
  (params (Move%20Target :type Vector))
  (Variables|Default|SetActive%20Command "NewEnumerator2")
  (AI|AIMoveTo self Move%20Target 0 5.0 false))

(event EventBeginPlay)

(event Collision|EventActorBeginOverlap
  (params (OtherActor :type Actor%20Object%20Reference)))

(event EventTick
  (params (DeltaSeconds :type Float%20%28single-precision%29)))

(fn ConstructionScript
  (|CallParentFunction))