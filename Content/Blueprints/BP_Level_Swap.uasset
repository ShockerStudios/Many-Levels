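; BP_Level_Swap is a trigger actor that moves the player to another level.
; When BP_Devvy overlaps LevelTrigger, it checks whether the player mesh's first material is M_FlatGreyLight_Inst, using the material as the pass condition.
; On a match, it copies the player's Score into the GI_Haunted game instance and opens the target Level.
; Otherwise, it shows a DoorNotWid widget and plays its UpAnim.
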(event OnComponentBeginOverlap(LevelTrigger)
  (params (OverlappedComponent :type Primitive%20Component%20Object%20Reference) (OtherActor :type Actor%20Object%20Reference) (OtherComp :type Primitive%20Component%20Object%20Reference) (OtherBodyIndex :type Integer) (bFromSweep :type Boolean) (SweepResult :type Hit%20Result%20Structure%20%28by%20ref%29))
  (bind _asbp_devvy (Utilities|Casting|CastToBP_Devvy OtherActor))
  (if (== (Rendering|Material|GetMaterial (Variables|/Script/Engine.Character|GetMesh _asbp_devvy) 0) "/Game/Assets/Materials/M_FlatGreyLight_Inst.M_FlatGreyLight_Inst")
    ;[0 1 0.7137] Prof - Setting the Game Instance Score from Player score
    (bind _asgi_haunted (Utilities|Casting|CastToGI_Haunted (Game|GetGameInstance)))
    (Variables|/Game/Blueprints/GI_Haunted.GI_Haunted_C|SetScore _asgi_haunted (Variables|/Game/Blueprints/BP_Devvy.BP_Devvy_C|GetScore _asbp_devvy))
    (Game|OpenLevel(byObjectReference) (Variables|Default|GetLevel))
    (else
      (bind _returnvalue (UserInterface|CreateWidget "/Game/Sapphire/Nicole/DoorNotWid.DoorNotWid_C" 0 self))
      (UserInterface|Viewport|AddtoViewport _returnvalue 0)
      (UserInterface|Animation|PlayAnimation _returnvalue (Variables|/Game/Sapphire/Nicole/DoorNotWid.DoorNotWid_C|GetUpAnim _returnvalue) 0.0 1 "Forward" 1.0 false))))

(event Collision|EventActorBeginOverlap
  (params (OtherActor :type Actor%20Object%20Reference)))

(event EventTick
  (params (DeltaSeconds :type Float%20%28single-precision%29)))

(fn ConstructionScript)