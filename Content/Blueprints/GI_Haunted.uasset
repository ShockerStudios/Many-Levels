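; GI_Haunted is a game instance Blueprint that manages a single music track at a time.
; PlaySpecificMusic stops the current track, then creates and plays a valid sound as 2D audio at a quarter of the requested volume, optionally persisting across level transitions.
; The new audio component is stored in CurrentMusic, which StopMusic checks for validity before stopping.
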(fn PlaySpecificMusic
  (params (Sound :type Sound%20Base%20Object%20Reference) (VolumeMultiplier :type Float%20%28single-precision%29) (Perists? :type Boolean))
  (CallFunction|StopMusic)
  (if (Utilities|IsValid Sound)
    (bind _returnvalue (Audio|CreateSound2D Sound (* VolumeMultiplier 0.25) 1.0 0.0 0 Perists?))
    (bind _output_get (Variables|MusicLoader|SetCurrentMusic _returnvalue))
    (Audio|Components|Audio|Play _output_get 0.0)))

(fn StopMusic
  (bind _currentmusic (Variables|MusicLoader|GetCurrentMusic))
  (if (Utilities|IsValid _currentmusic)
    (Audio|Components|Audio|Stop _currentmusic)))