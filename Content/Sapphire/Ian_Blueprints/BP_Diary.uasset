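; BP_Diary is an interactable diary that shows its entry text in an on-screen widget.
; A text render becomes visible while BP_Devvy overlaps the Box trigger.
; Interact creates a UI_DiaryEntry widget filled with InText, guarded by a DoOnce so it opens only once.
; Leaving the box hides the text render, removes the widget and resets the DoOnce.
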(event OnComponentBeginOverlap(Box)
  (params (OverlappedComponent :type Primitive%20Component%20Object%20Reference) (OtherActor :type Actor%20Object%20Reference) (OtherComp :type Primitive%20Component%20Object%20Reference) (OtherBodyIndex :type Integer) (bFromSweep :type Boolean) (SweepResult :type Hit%20Result%20Structure%20%28by%20ref%29))
  (Utilities|Casting|CastToBP_Devvy OtherActor)
  (Rendering|SetVisibility (Variables|Default|GetTextRender) true false))

(event OnComponentEndOverlap(Box)
  (params (OverlappedComponent :type Primitive%20Component%20Object%20Reference) (OtherActor :type Actor%20Object%20Reference) (OtherComp :type Primitive%20Component%20Object%20Reference) (OtherBodyIndex :type Integer))
  (bind _w_diary (Variables|Default|GetW_Diary))
  (Utilities|Casting|CastToBP_Devvy OtherActor)
  (Rendering|SetVisibility (Variables|Default|GetTextRender) false false)
  (CallFunction|ResetInteraction)
  (Utilities|IsValid _w_diary
    (:Is%20Valid
      (Widget|RemovefromParent _w_diary))))

(event Custom|ResetInteraction
  (Utilities|FlowControl|DoOnce false) ; enters at Reset
)

(event EventInteract
  (Utilities|FlowControl|DoOnce false
    (:Completed
      (bind _returnvalue (UserInterface|CreateWidget "/Game/Sapphire/Ian_Blueprints/UI_DiaryEntry.UI_DiaryEntry_C"))
      (bind _output_get (Variables|Default|SetW_Diary _returnvalue))
      (Rendering|Components|TextRender|SetText (Variables|/Game/Sapphire/Ian_Blueprints/UI_DiaryEntry.UI_DiaryEntry_C|GetText _output_get) (Variables|Default|GetIn%20Text))
      (UserInterface|Viewport|AddtoViewport _output_get 0))))

(fn ConstructionScript)