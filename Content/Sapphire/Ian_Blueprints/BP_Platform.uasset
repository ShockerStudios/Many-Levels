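; BP_Platform is a moving platform actor that animates its Cube component's relative location along timeline tracks.
; BeginPlay starts the Moving timeline when StartPlatform is set, while the MovePlatform event prints a debug string and plays a separate Timeline_0.
; Each timeline's Update moves the Cube without sweep, then runs a six-second Delay that toggles the shared Loop flag to alternate reverse and forward playback.
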(event Custom|Move%20Platform
  (Development|PrintString "Hello")
  (bind _newtrack_2 (Timeline|Timeline_0 Play)
    (:Update
      (Transformation|SetRelativeLocation (Variables|Default|GetCube) _newtrack_2 false false)
      (Utilities|FlowControl|Delay 6.0)
      (if (Variables|Default|GetLoop)
        (Variables|Default|SetLoop false)
        (Timeline|Timeline_0 Reverse)
        (else
          (Variables|Default|SetLoop true)
          (Timeline|Timeline_0 Play))))))

(event EventBeginPlay
  (if (Variables|Default|GetStart%20Platform)
    (bind _newtrack_2 (Timeline|Moving Play)
      (:Update
        (Transformation|SetRelativeLocation (Variables|Default|GetCube) _newtrack_2 false false)
        (Utilities|FlowControl|Delay 6.0)
        (if (Variables|Default|GetLoop)
          (Variables|Default|SetLoop false)
          (Timeline|Moving Reverse)
          (else
            (Variables|Default|SetLoop true)
            (Timeline|Moving Play)))))))

(event Collision|EventActorBeginOverlap
  (params (OtherActor :type Actor%20Object%20Reference)))

(event EventTick
  (params (DeltaSeconds :type Float%20%28single-precision%29)))

(fn ConstructionScript)