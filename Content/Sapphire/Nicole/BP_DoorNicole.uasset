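; BP_DoorNicole is a two-panel door that snaps between open and closed poses.
; Its Open and Close events set fixed relative rotations on two static mesh components, swinging them in opposite directions.
; The rotations are instant, with no timeline or interpolation, and nothing in its graphs triggers the events, so they rely on outside callers.
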(event Custom|Open
  (Utilities|FlowControl|Sequence
    (:then_0
      (Transformation|SetRelativeRotation (Variables|Default|GetStaticMesh) "0,140.000000, 0" false false))
    (:then_1
      (Transformation|SetRelativeRotation (Variables|Default|GetStaticMesh1) "0,40.000000, 0" false false))))

(event Custom|Close
  (Utilities|FlowControl|Sequence
    (:then_0
      (Transformation|SetRelativeRotation (Variables|Default|GetStaticMesh) "0,0.000000, 0" false false))
    (:then_1
      (Transformation|SetRelativeRotation (Variables|Default|GetStaticMesh1) "0,180.000000, 0" false false))))

(fn ConstructionScript)