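; BP_Breakable_Timed is a breakable object that restores itself after a timed delay.
; Its Destroy event runs the parent's destroy logic, then reveals the Box component for the length of Duration.
; When the delay ends, it makes the static mesh visible again, re-enables query and physics collision, and hides the Box.
; The construction script only calls the parent's.
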(event EventDestroy
  (bind _staticmesh (Variables|Default|GetStaticMesh))
  (|CallParentFunction)
  (Development|SetHiddeninGame (Variables|Default|GetBox) false false)
  (Utilities|FlowControl|Delay (Variables|Default|GetDuration))
  (Rendering|SetVisibility _staticmesh true false)
  (Collision|SetCollisionEnabled _staticmesh "QueryAndPhysics")
  (Development|SetHiddeninGame (Variables|Default|GetBox) true false))

(fn ConstructionScript
  (|CallParentFunction))