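; A platform that falls shortly after BP_Devvy steps into its trigger box, then respawns at its starting spot.
; Tick drops it by a fixed per-frame offset with teleport and no sweep while Falling is set, so speed depends on frame rate.
; When a second box overlaps anything other than Devvy, it stops, hides and disables both meshes' collision, then restores them at the saved location after a delay.
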(event OnComponentBeginOverlap(Box)
  (params (OverlappedComponent :type Primitive%20Component%20Object%20Reference) (OtherActor :type Actor%20Object%20Reference) (OtherComp :type Primitive%20Component%20Object%20Reference) (OtherBodyIndex :type Integer) (bFromSweep :type Boolean) (SweepResult :type Hit%20Result%20Structure%20%28by%20ref%29))
  (Utilities|Casting|CastToBP_Devvy OtherActor)
  (Utilities|FlowControl|Delay 0.2)
  (Variables|Default|SetFalling true))

(event OnComponentBeginOverlap(Box1)
  (params (OverlappedComponent :type Primitive%20Component%20Object%20Reference) (OtherActor :type Actor%20Object%20Reference) (OtherComp :type Primitive%20Component%20Object%20Reference) (OtherBodyIndex :type Integer) (bFromSweep :type Boolean) (SweepResult :type Hit%20Result%20Structure%20%28by%20ref%29))
  (Utilities|Casting|CastToBP_Devvy OtherActor
    (:CastFailed
      (Variables|Default|SetFalling false)
      (Rendering|SetActorHiddenInGame true)
      (Collision|SetCollisionEnabled (Variables|Default|GetStaticMesh1) "NoCollision")
      (Collision|SetCollisionEnabled (Variables|Default|GetStaticMesh) "NoCollision")
      (Utilities|FlowControl|Delay 1.0)
      (Transformation|SetActorLocation (Variables|Default|GetStartLocation) false true)
      (Rendering|SetActorHiddenInGame false)
      (Collision|SetCollisionEnabled (Variables|Default|GetStaticMesh1) "QueryAndPhysics")
      (Collision|SetCollisionEnabled (Variables|Default|GetStaticMesh) "QueryAndPhysics"))))

(event EventBeginPlay
  (Variables|Default|SetStartLocation (Transformation|GetActorLocation)))

(event EventTick
  (params (DeltaSeconds :type Float%20%28single-precision%29))
  (if (Variables|Default|GetFalling)
    (Transformation|AddActorLocalOffset "0, 0,-8.000000" false true)))

(fn ConstructionScript)