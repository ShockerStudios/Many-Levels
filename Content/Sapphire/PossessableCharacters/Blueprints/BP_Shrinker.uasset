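; BP_Shrinker is a possessable character that toggles between normal and shrunken size when F is pressed.
; Each toggle plays a sound and rescales the actor, its gravity, jump, walk speed and camera boom to match.
; The GrowCheck overlap component tracks a single Obstacle reference, cleared on any end overlap; while it is valid, growing is refused with a No_Grow sound.
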(event OnComponentBeginOverlap(GrowCheck)
  (params (OverlappedComponent :type Primitive%20Component%20Object%20Reference) (OtherActor :type Actor%20Object%20Reference) (OtherComp :type Primitive%20Component%20Object%20Reference) (OtherBodyIndex :type Integer) (bFromSweep :type Boolean) (SweepResult :type Hit%20Result%20Structure%20%28by%20ref%29))
  (Utilities|IsValid OtherActor
    (:Is%20Valid
      (Variables|Default|SetObstacle OtherActor))))

(event OnComponentEndOverlap(GrowCheck)
  (params (OverlappedComponent :type Primitive%20Component%20Object%20Reference) (OtherActor :type Actor%20Object%20Reference) (OtherComp :type Primitive%20Component%20Object%20Reference) (OtherBodyIndex :type Integer))
  (Utilities|IsValid OtherActor
    (:Is%20Valid
      (Variables|Default|SetObstacle 0))))

(event EventBeginPlay
  (|CallParentFunction) ; This node is disabled and will not be called.\nDrag off pins to build functionality.
)

(event Collision|EventActorBeginOverlap
  (params (OtherActor :type Actor%20Object%20Reference)))

(event EventTick
  (params (DeltaSeconds :type Float%20%28single-precision%29))
  (|CallParentFunction DeltaSeconds))

(event Input|KeyboardEvents|F
  (params (Key :type Key%20Structure :default "None"))
  (bind _self self)
  (bind _charactermovement (Variables|Character|GetCharacterMovement))
  (bind _springarm (Variables|Default|GetSpringArm))
  (:Pressed
    (if (Variables|Default|GetShrunk)
      (Utilities|IsValid (Variables|Default|GetObstacle)
        (:Is%20Valid
          (Audio|PlaySound2D "/Game/Sapphire/_Alex/Audio/No_Grow.No_Grow" 1.0 1.0 0.0 0 0))
        (:Is%20Not%20Valid
          (Audio|PlaySound2D "/Game/Jade/Sounds_Jade/CAFOFO_RPGSounds/DungeonElements/Arrow_Release_2.Arrow_Release_2" 1.0 1.0 0.0 0 0)
          (Variables|Default|SetShrunk false)
          (Transformation|SetActorScale3D _self "1.000000,1.000000,1.000000")
          (Variables|/Script/Engine.CharacterMovementComponent|SetGravityScale _charactermovement 4.0)
          (Variables|/Script/Engine.CharacterMovementComponent|SetJumpZVelocity _charactermovement 1.2e+03)
          (Variables|/Script/Engine.CharacterMovementComponent|SetMaxWalkSpeed _charactermovement 6e+02)
          (Variables|/Script/Engine.SpringArmComponent|SetTargetArmLength _springarm 6e+02)
          (Variables|/Script/Engine.SpringArmComponent|SetSocketOffset _springarm "0, 0, 0")))
      (else
        (Audio|PlaySound2D "/Game/Jade/Sounds_Jade/CAFOFO_RPGSounds/DungeonElements/Arrow_Release_1.Arrow_Release_1" 1.0 1.0 0.0 0 0)
        (Variables|Default|SetShrunk true)
        (Transformation|SetActorScale3D _self "0.200000,0.200000,0.200000")
        (Variables|/Script/Engine.CharacterMovementComponent|SetGravityScale _charactermovement 1.0)
        (Variables|/Script/Engine.CharacterMovementComponent|SetJumpZVelocity _charactermovement 3e+02)
        (Variables|/Script/Engine.CharacterMovementComponent|SetMaxWalkSpeed _charactermovement 1.5e+02)
        (Variables|/Script/Engine.SpringArmComponent|SetTargetArmLength _springarm 1.5e+02)
        (Variables|/Script/Engine.SpringArmComponent|SetSocketOffset _springarm "0, 0, 0")))))

(fn ConstructionScript
  (|CallParentFunction))