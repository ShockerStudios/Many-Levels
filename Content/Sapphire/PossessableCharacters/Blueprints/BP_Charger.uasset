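; BP_Charger is a possessable character whose Jump input triggers a forward charge that smashes BP_Breakable actors.
; Charging disables input, loops a sprint animation and repeatedly launches the character forward on a counted delay loop.
; A hit above roughly foot height maxes the counter to end the charge early, destroying any breakable struck.
; Either ending plays a wall-impact animation through a DoOnce, then restores the animation Blueprint, input and charge ability.
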(event Custom|Charge
  (bind _returnvalue (Transformation|GetActorForwardVector))
  (bind _mesh (Variables|Character|GetMesh))
  ;[1 1 1] Charging
  (Variables|Default|SetCanCharge false)
  (Input|DisableInput (Game|GetPlayerController 0))
  (Components|Animation|PlayAnimation (Variables|Character|GetMesh) "/Game/Sapphire/PossessableCharacters/Animations/Charger_Alert_Sprint.Charger_Alert_Sprint" true)
  (Character|LaunchCharacter (Math|Vector|MakeVector (* (.x _returnvalue) 1.6e+03) (* (.y _returnvalue) 1.6e+03) 0.0) false false :!label _label)
  (Utilities|FlowControl|Delay 0.08)
  (Math|Integer|IncrementInt (Variables|Default|GetChargeStop)
    (:%20%20
      (if (>= (Variables|Default|GetChargeStop) 30)
        (Utilities|FlowControl|DoOnce false :!label _label_2
          (:Completed
            (Components|Animation|PlayAnimation _mesh "/Game/Sapphire/PossessableCharacters/Animations/Charger_Alert_ChargeWall.Charger_Alert_ChargeWall" false)
            (Components|Movement|StopMovementImmediately (Variables|Character|GetCharacterMovement))
            (Utilities|FlowControl|Delay 0.5)
            (Components|Animation|SetAnimationMode _mesh "AnimationBlueprint")
            (Input|EnableInput (Game|GetPlayerController 0))
            (Variables|Default|SetCanCharge true)
            (Variables|Default|SetChargeStop 0)
            (goto _label_2 Reset)))
        (else
          (goto _label))))))

(event Custom|StopCharging
  (bind _returnvalue (Transformation|GetActorForwardVector))
  (bind _mesh (Variables|Character|GetMesh))
  ;[1 1 1] Charging
  (Variables|Default|SetChargeStop 31)
  (if (>= (Variables|Default|GetChargeStop) 30) :!label _label
    (Utilities|FlowControl|DoOnce false :!label _label_2
      (:Completed
        (Components|Animation|PlayAnimation _mesh "/Game/Sapphire/PossessableCharacters/Animations/Charger_Alert_ChargeWall.Charger_Alert_ChargeWall" false)
        (Components|Movement|StopMovementImmediately (Variables|Character|GetCharacterMovement))
        (Utilities|FlowControl|Delay 0.5)
        (Components|Animation|SetAnimationMode _mesh "AnimationBlueprint")
        (Input|EnableInput (Game|GetPlayerController 0))
        (Variables|Default|SetCanCharge true)
        (Variables|Default|SetChargeStop 0)
        (goto _label_2 Reset)))
    (else
      (Character|LaunchCharacter (Math|Vector|MakeVector (* (.x _returnvalue) 1.6e+03) (* (.y _returnvalue) 1.6e+03) 0.0) false false)
      (Utilities|FlowControl|Delay 0.08)
      (Math|Integer|IncrementInt (Variables|Default|GetChargeStop)
        (:%20%20
          (goto _label))))))

(event EventBeginPlay
  (|CallParentFunction) ; This node is disabled and will not be called.\nDrag off pins to build functionality.
)

(event Collision|EventActorBeginOverlap
  (params (OtherActor :type Actor%20Object%20Reference)))

(event EventTick
  (params (DeltaSeconds :type Float%20%28single-precision%29))
  (|CallParentFunction DeltaSeconds) ; This node is disabled and will not be called.\nDrag off pins to build functionality.
)

(event Collision|EventHit
  (params (MyComp :type Primitive%20Component%20Object%20Reference) (Other :type Actor%20Object%20Reference) (OtherComp :type Primitive%20Component%20Object%20Reference) (bSelfMoved :type Boolean) (HitLocation :type Vector :default "0, 0, 0") (HitNormal :type Vector :default "0, 0, 0") (NormalImpulse :type Vector :default "0, 0, 0") (Hit :type Hit%20Result%20Structure%20%28by%20ref%29))
  (if (> (+ (.z HitLocation) 0.6) (- (.z (Transformation|GetActorLocation self)) 71.0))
    (if (not (Variables|Default|GetCanCharge))
      (CallFunction|StopCharging)
      (bind _asbp_breakable (Utilities|Casting|CastToBP_Breakable Other))
      (Default|Destroy _asbp_breakable))))

(event Input|ActionEvents|InputActionJump
  (params (Key :type Key%20Structure :default "None"))
  (:Pressed
    (if (Variables|Default|GetCanCharge)
      (CallFunction|Charge))))

(fn ConstructionScript
  (|CallParentFunction))