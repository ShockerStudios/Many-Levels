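; BP_FallBound is a trigger box that catches BP_Devvy, likely after a fall, and sends it back to a respawn point.
; On BeginPlay it searches all BP_SpawnPoint actors and caches the one whose RespawnType matches its FallType, keeping the last match.
; When BP_Devvy overlaps the box, it moves to that point's Location and one of two random 2D sounds plays.
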(event OnComponentBeginOverlap(Box)
  (params (OverlappedComponent :type Primitive%20Component%20Object%20Reference) (OtherActor :type Actor%20Object%20Reference) (OtherComp :type Primitive%20Component%20Object%20Reference) (OtherBodyIndex :type Integer) (bFromSweep :type Boolean) (SweepResult :type Hit%20Result%20Structure%20%28by%20ref%29))
  (bind _asbp_devvy (Utilities|Casting|CastToBP_Devvy OtherActor))
  (Transformation|SetActorLocation _asbp_devvy (Variables|/Game/Sapphire/_Alex/Blueprints/BP_SpawnPoint.BP_SpawnPoint_C|GetLocation (Variables|Default|GetBP_Respawn)) false false)
  (Audio|SpawnSound2D (Utilities|Array|Get(acopy) (Variables|Default|GetSound) (Math|Random|RandomInteger 2)) 1.0 1.0 0.0 0))

(event EventBeginPlay
  (bind _outactors (Actor|GetAllActorsOfClass "/Game/Sapphire/_Alex/Blueprints/BP_SpawnPoint.BP_SpawnPoint_C"))
  (for _array_element _outactors
    (if (== (Variables|/Game/Sapphire/_Alex/Blueprints/BP_SpawnPoint.BP_SpawnPoint_C|GetRespawnType _array_element) (Variables|Default|GetFallType))
      (Variables|Default|SetBP_Respawn _array_element))))

(fn ConstructionScript)