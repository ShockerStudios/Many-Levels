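; BP_AudioPlayer is a trigger volume that plays a 2D sound once, when BP_Devvy first enters its box while it is active.
; On firing, it calls ToggleActive on the stored audio component of every BP_AudioPlayer, then spawns and stores its own sound.
; It then activates the players in AllowOtherSounds and deactivates those in TurnOffOtherSounds, gating which triggers can fire next.
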(event OnComponentBeginOverlap(Box)
  (params (OverlappedComponent :type Primitive%20Component%20Object%20Reference) (OtherActor :type Actor%20Object%20Reference) (OtherComp :type Primitive%20Component%20Object%20Reference) (OtherBodyIndex :type Integer) (bFromSweep :type Boolean) (SweepResult :type Hit%20Result%20Structure%20%28by%20ref%29))
  (Utilities|Casting|CastToBP_Devvy OtherActor)
  (if (Variables|Default|GetActive?)
    (Utilities|FlowControl|DoOnce false
      (:Completed
        (bind _outactors (Actor|GetAllActorsOfClass "BP_AudioPlayer_C"))
        (for _array_element _outactors
          (Utilities|IsValid (Variables|BP_AudioPlayer_C|GetStopAudio _array_element)
            (:Is%20Valid
              (Components|Activation|ToggleActive (Variables|BP_AudioPlayer_C|GetStopAudio _array_element)))))
        (bind _returnvalue (Audio|SpawnSound2D (Variables|Default|GetSound) 1.0 1.0 0.0 0))
        (Variables|Default|SetStopAudio _returnvalue)
        (for _array_element_2 (Variables|Default|GetAllowOtherSounds)
          (Utilities|IsValid _array_element_2
            (:Is%20Valid
              (CallFunction|Activate _array_element_2))))
        (for _array_element_3 (Variables|Default|GetTurnOffOtherSounds)
          (Utilities|IsValid _array_element_3
            (:Is%20Valid
              (CallFunction|Deactivate _array_element_3))))))))

(event Custom|Activate
  (Variables|Default|SetActive? true))

(event Custom|Deactivate
  (Variables|Default|SetActive? false))

(fn ConstructionScript)