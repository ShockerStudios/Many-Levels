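; BP_Button is a pressure-style trigger that temporarily reveals hidden keys when BP_Devvy overlaps its box.
; It unhides and enables collision on every BP_Key whose KeyType matches ButtonType, optionally playing a level sequence cutscene the first time.
; After a delay it hides and disables only the last matched key, if still valid, then resets the DoOnce gate to re-arm.
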(event OnComponentBeginOverlap(Box)
  (params (OverlappedComponent :type Primitive%20Component%20Object%20Reference) (OtherActor :type Actor%20Object%20Reference) (OtherComp :type Primitive%20Component%20Object%20Reference) (OtherBodyIndex :type Integer) (bFromSweep :type Boolean) (SweepResult :type Hit%20Result%20Structure%20%28by%20ref%29))
  (Utilities|Casting|CastToBP_Devvy OtherActor)
  (Audio|PlaySound2D "/Game/Jade/Sounds_Jade/CAFOFO_RPGSounds/DungeonElements/Switch_and_Lever_1_1.Switch_and_Lever_1_1" 1.0 1.0 0.0 0 0)
  (Utilities|FlowControl|DoOnce false :!label _label
    (:Completed
      (bind _outactors (Actor|GetAllActorsOfClass "/Game/Sapphire/_Alex/Blueprints/BP_Key.BP_Key_C"))
      (for _array_element _outactors
        (Utilities|IsValid _array_element
          (:Is%20Valid
            (if (== (Variables|/Game/Sapphire/_Alex/Blueprints/BP_Key.BP_Key_C|GetKeyType _array_element) (Variables|Default|GetButtonType))
              (bind _output_get (Variables|Default|SetAs%20BP%20Key _array_element))
              (Collision|SetCollisionEnabled (Variables|/Game/Sapphire/_Alex/Blueprints/BP_Key.BP_Key_C|GetSphere _output_get) "QueryAndPhysics")
              (Rendering|SetActorHiddenInGame _output_get false)))))
      (if (Variables|Default|GetPlayCutscene?)
        (Variables|Default|SetPlayCutscene? false)
        (Sequencer|Player|Play (Variables|Default|GetButtonVideo) :!class /Script/MovieScene.MovieSceneSequencePlayer)
        (Utilities|FlowControl|Delay 4.0))
      (Utilities|FlowControl|Delay 4.0)
      (Utilities|IsValid (Variables|Default|GetAs%20BP%20Key)
        (:Is%20Valid
          (Collision|SetCollisionEnabled (Variables|/Game/Sapphire/_Alex/Blueprints/BP_Key.BP_Key_C|GetSphere (Variables|Default|GetAs%20BP%20Key)) "NoCollision")
          (Rendering|SetActorHiddenInGame (Variables|Default|GetAs%20BP%20Key) true)
          (Audio|PlaySound2D "/Game/Jade/Sounds_Jade/CAFOFO_RPGSounds/DungeonElements/Switch_and_Lever_6_4.Switch_and_Lever_6_4" 1.0 1.0 0.0 0 0)
          (goto _label Reset))))))

(event EventBeginPlay
  (bind _returnvalue (Sequencer|Player|CreateLevelSequencePlayer "/Game/Sapphire/_Alex/Scenes/Key.Key"))
  (Variables|Default|SetButtonVideo _returnvalue)
  (bind _returnvalue_2 (Actor|GetActorOfClass "/Game/Blueprints/BP_Devvy.BP_Devvy_C"))
  (Variables|Default|SetTarget _returnvalue_2))

(fn ConstructionScript)