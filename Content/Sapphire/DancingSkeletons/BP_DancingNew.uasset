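; A dancing skeleton collectible that BP_Devvy picks up, after which it follows the player.
; Overlapping its Pickup component adds score, plays a sound, turns the mesh gold, destroys the trigger and starts following.
; A self-repeating, delay-paced AIMoveTo loop chases the player beyond a set distance, teleporting to them if stationary, and otherwise halts by targeting itself.
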(event OnComponentBeginOverlap(Pickup)
  (params (OverlappedComponent :type Primitive%20Component%20Object%20Reference) (OtherActor :type Actor%20Object%20Reference) (OtherComp :type Primitive%20Component%20Object%20Reference) (OtherBodyIndex :type Integer) (bFromSweep :type Boolean) (SweepResult :type Hit%20Result%20Structure%20%28by%20ref%29))
  (Utilities|Casting|CastToBP_Devvy OtherActor)
  (bind _outactors (Actor|GetAllActorsOfClass "/Game/Blueprints/BP_Devvy.BP_Devvy_C"))
  (for _array_element _outactors
    (Variables|/Game/Blueprints/BP_Devvy.BP_Devvy_C|SetScore _array_element (+ (Variables|/Game/Blueprints/BP_Devvy.BP_Devvy_C|GetScore _array_element) 10)))
  (Audio|PlaySound2D "/Game/Sapphire/_Alex/Audio/PickupSkeleton.PickupSkeleton" 1.0 1.0 0.0 0 0)
  (Rendering|Material|SetMaterial (Variables|Character|GetMesh) 0 "/Game/Sapphire/_Alex/Materials/M_GoldSkeleton.M_GoldSkeleton")
  (Variables|Default|SetFollow%20Player? true)
  (Components|DestroyComponent (Variables|Default|GetPickup))
  (CallFunction|FollowPlayer))

(event Custom|StopMovement
  ;[1 1 1] Always Following
  (AI|AIMoveTo self "0, 0, 0" self 5.0 false
    (:then
      (Utilities|FlowControl|Delay 0.2)
      (CallFunction|FollowPlayer))))

(event Custom|Follow%20Player
  ;[1 1 1] Always Following
  (if (Variables|Default|GetFollow%20Player?)
    (if (>= (Transformation|GetDistanceTo (Variables|Default|GetCharacter%20Ref)) 3e+02)
      (AI|AIMoveTo self "0, 0, 0" (Variables|Default|GetCharacter%20Ref) 5.0 false
        (:then
          (Utilities|FlowControl|Delay 0.2)
          (if (Utilities|Operators|EqualEqual :A (Transformation|GetVelocity self) :ErrorTolerance 0.0)
            (Transformation|Teleport (Transformation|GetActorLocation (Variables|Default|GetCharacter%20Ref)) "0, 0, 0"))))
      (else
        (AI|AIMoveTo self "0, 0, 0" self 5.0 false
          (:then
            _))))
    (Utilities|FlowControl|Delay 0.2)
    (CallFunction|FollowPlayer)))

(event EventBeginPlay
  (|CallParentFunction)
  (bind _asbp_devvy (Utilities|Casting|CastToBP_Devvy (Game|GetPlayerCharacter 0)))
  (Variables|Default|SetCharacter%20Ref _asbp_devvy))

(fn ConstructionScript)