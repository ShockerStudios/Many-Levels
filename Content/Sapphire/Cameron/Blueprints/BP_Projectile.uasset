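; BP_Projectile is a hazard that sends a BP_Devvy actor back to a spawn point when it touches the Projectile component.
; On BeginPlay it caches the BP_SpawnPoint whose RespawnType matches its SpawnID.
; On overlap it debug-prints the touched component's name and teleports the actor unless that name ends in "Nah".
; If the teleported actor is also a BP_Shrinker, its Obstacle reference is cleared.
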(event OnComponentBeginOverlap(Projectile)
  (params (OverlappedComponent :type Primitive%20Component%20Object%20Reference) (OtherActor :type Actor%20Object%20Reference) (OtherComp :type Primitive%20Component%20Object%20Reference) (OtherBodyIndex :type Integer) (bFromSweep :type Boolean) (SweepResult :type Hit%20Result%20Structure%20%28by%20ref%29))
  (bind _returnvalue (Utilities|GetDisplayName OtherComp))
  (bind _asbp_devvy (Utilities|Casting|CastToBP_Devvy OtherActor))
  (Development|PrintString _returnvalue)
  (if (not (Utilities|Enum|Equal(Enum) (Utilities|String|Right _returnvalue 3) "Nah"))
    (Transformation|SetActorLocation _asbp_devvy (Variables|/Game/Sapphire/_Alex/Blueprints/BP_SpawnPoint.BP_SpawnPoint_C|GetLocation (Variables|Default|GetSpawnPoint)) false false)
    (bind _asbp_shrinker (Utilities|Casting|CastToBP_Shrinker OtherActor))
    (Variables|/Game/Sapphire/PossessableCharacters/Blueprints/BP_Shrinker.BP_Shrinker_C|SetObstacle _asbp_shrinker 0)))

(event EventBeginPlay
  (bind _outactors (Actor|GetAllActorsOfClass "/Game/Sapphire/_Alex/Blueprints/BP_SpawnPoint.BP_SpawnPoint_C"))
  (for _array_element _outactors
    (if (== (Variables|/Game/Sapphire/_Alex/Blueprints/BP_SpawnPoint.BP_SpawnPoint_C|GetRespawnType _array_element) (Variables|Default|GetSpawnID))
      (Variables|Default|SetSpawnPoint _array_element))))

(fn ConstructionScript)