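; Sound manager that holds the background music and plays voice lines over it.
; On BeginPlay it assigns the Dancing Skeletons track to the Song component; its explicit Play call is unconnected.
; PlaySound assigns the given sound to VoiceLine and activates it, ducking Song to half volume.
; A Delay matching the clip's duration then restores full music volume, with no handling for overlapping calls.
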(event Custom|Play%20Sound
  (params (NewSound :type Sound%20Base%20Object%20Reference))
  (bind _voiceline (Variables|Default|GetVoiceLine))
  (bind _song (Variables|Default|GetSong))
  (Audio|Components|Audio|SetSound _voiceline NewSound)
  (Components|Activation|Activate _voiceline false)
  (Audio|Components|Audio|SetVolumeMultiplier _song 0.5 :!class /Script/Engine.AudioComponent)
  (Utilities|FlowControl|Delay (Variables|/Script/Engine.SoundBase|GetDuration NewSound))
  (Audio|Components|Audio|SetVolumeMultiplier _song 1.0 :!class /Script/Engine.AudioComponent))

(event EventBeginPlay
  (Audio|Components|Audio|SetSound (Variables|Default|GetSong) "/Game/Sapphire/Cameron/2020-10-26_-_Dancing_Skeletons_-_www_FesliyanStudios_com_Steve_Oxen.2020-10-26_-_Dancing_Skeletons_-_www_FesliyanStudios_com_Steve_Oxen"))

(fn ConstructionScript)