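; BP_SecretShelf is a shelf that slides to a hidden destination when the BP_Devvy character walks into its trigger box.
; On BeginPlay it finds the MoveDestination actor whose MatchNum equals its Number and stores that location.
; Overlap plays the MoveShelf timeline, which lerps from the shelf's current location toward the stored point each update, so the motion eases rather than being linear.
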(event OnComponentBeginOverlap(Box)
  (params (OverlappedComponent :type Primitive%20Component%20Object%20Reference) (OtherActor :type Actor%20Object%20Reference) (OtherComp :type Primitive%20Component%20Object%20Reference) (OtherBodyIndex :type Integer) (bFromSweep :type Boolean) (SweepResult :type Hit%20Result%20Structure%20%28by%20ref%29))
  (Utilities|Casting|CastToBP_Devvy OtherActor)
  (bind _newtrack_0 (Timeline|MoveShelf Play)
    (:Update
      (Transformation|SetActorLocation (Math|Vector|Lerp(Vector) (Transformation|GetActorLocation) (Variables|Default|GetDestination) _newtrack_0) false false))))

(event EventBeginPlay
  (bind _outactors (Actor|GetAllActorsOfClass "/Game/Sapphire/Cameron/Blueprints/MoveDestination.MoveDestination_C"))
  (for _array_element _outactors
    (if (== (Variables|/Game/Sapphire/Cameron/Blueprints/MoveDestination.MoveDestination_C|GetMatchNum _array_element) (Variables|Default|GetNumber))
      (Variables|Default|SetDestination (Transformation|GetActorLocation _array_element)))))

(fn ConstructionScript)