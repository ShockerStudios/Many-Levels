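; BP_BlockWall is a toggleable wall for a block-pushing mechanic, with a direction-dependent blocking volume.
; WallToggle flips Active, switching Wall collision and material, and enables BlockWall collision on activation only if the direction check passes.
; Enter and Exit overlap components set CanGrab on BP_BlockPusher to true and false respectively, printing debug text.
; Wall collision starts disabled at BeginPlay.
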(event OnComponentBeginOverlap(Enter)
  (params (OverlappedComponent :type Primitive%20Component%20Object%20Reference) (OtherActor :type Actor%20Object%20Reference) (OtherComp :type Primitive%20Component%20Object%20Reference) (OtherBodyIndex :type Integer) (bFromSweep :type Boolean) (SweepResult :type Hit%20Result%20Structure%20%28by%20ref%29))
  ;[1 1 1] Set Grabbing Mode
  (bind _asbp_third_person_character (Utilities|Casting|CastToBP_BlockPusher OtherActor))
  (Variables|/Game/Sapphire/Cameron/Blueprints/BP_BlockPusher.BP_BlockPusher_C|SetCanGrab _asbp_third_person_character true)
  (Development|PrintString "CanGrab"))

(event OnComponentBeginOverlap(Exit)
  (params (OverlappedComponent :type Primitive%20Component%20Object%20Reference) (OtherActor :type Actor%20Object%20Reference) (OtherComp :type Primitive%20Component%20Object%20Reference) (OtherBodyIndex :type Integer) (bFromSweep :type Boolean) (SweepResult :type Hit%20Result%20Structure%20%28by%20ref%29))
  ;[1 1 1] Set Grabbing Mode
  (bind _asbp_third_person_character (Utilities|Casting|CastToBP_BlockPusher OtherActor))
  (Variables|/Game/Sapphire/Cameron/Blueprints/BP_BlockPusher.BP_BlockPusher_C|SetCanGrab _asbp_third_person_character false)
  (Development|PrintString "NoGrab"))

(event Custom|WallToggle
  (params (Direction :type Integer%20%28by%20ref%29))
  (bind _wall (Variables|Default|GetWall))
  (bind _blockwall (Variables|Default|GetBlockWall))
  ;[1 1 1] Toggle Wall
  (if (Variables|Default|GetActive)
    (Variables|Default|SetActive false)
    (Collision|SetCollisionEnabled _wall "NoCollision")
    (Rendering|Material|SetMaterial _wall 0 0)
    (Collision|SetCollisionEnabled _blockwall "NoCollision")
    (else
      (Variables|Default|SetActive true)
      (Collision|SetCollisionEnabled _wall "QueryAndPhysics")
      (Rendering|Material|SetMaterial _wall 0 0)
      (if (== Direction (Variables|Default|GetDirection))
        (Collision|SetCollisionEnabled _blockwall "QueryAndPhysics")))))

(event EventBeginPlay
  (Collision|SetCollisionEnabled (Variables|Default|GetWall) "NoCollision"))

(fn ConstructionScript)