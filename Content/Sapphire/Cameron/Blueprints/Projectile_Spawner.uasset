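; Projectile spawner that sends one reused projectile repeatedly toward a paired end point.
; On BeginPlay it picks the BP_ProjectileEnd whose Channel matches MatchyMatchyNumby, then spawns the projectile after SpawnDelay.
; A timeline lerps the projectile to that destination, while chained delays off its update return it to the spawner and call Loop to replay.
; EndLoop destroys the spawned projectile.
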(event Custom|Loop
  (bind _newtrack_0 (Timeline|Timeline_0 PlayFromStart)
    (:Update
      (Transformation|SetActorLocation (stale EventBeginPlay _returnvalue) (Math|Vector|Lerp(Vector) (Transformation|GetActorLocation) (Transformation|GetActorLocation (Variables|Default|GetDestination)) _newtrack_0) false false)
      (Utilities|FlowControl|Delay 5.0)
      (Transformation|SetActorLocation (stale EventBeginPlay _returnvalue) (Transformation|GetActorLocation) false false)
      (Utilities|FlowControl|Delay 0.2)
      (CallFunction|Loop))))

(event Custom|End%20Loop
  (Actor|DestroyActor (Variables|Default|GetSpawned%20Projectile)))

(event EventBeginPlay
  (bind _outactors (Actor|GetAllActorsOfClass "/Game/Sapphire/Cameron/Blueprints/BP_ProjectileEnd.BP_ProjectileEnd_C"))
  (for _array_element _outactors
    (if (== (Variables|/Game/Sapphire/Cameron/Blueprints/BP_ProjectileEnd.BP_ProjectileEnd_C|GetChannel _array_element) (Variables|Default|GetMatchyMatchyNumby))
      (Variables|Default|SetDestination _array_element)))
  (Utilities|FlowControl|Delay (Variables|Default|GetSpawn%20Delay))
  (bind _returnvalue (Game|SpawnActorfromClass (Variables|Default|GetProjectile%20) (Transformation|GetActorTransform) "Undefined" 0 0))
  (Variables|Default|SetSpawned%20Projectile _returnvalue)
  (bind _newtrack_0 (Timeline|Timeline_0 PlayFromStart)
    (:Update
      (Transformation|SetActorLocation _returnvalue (Math|Vector|Lerp(Vector) (Transformation|GetActorLocation) (Transformation|GetActorLocation (Variables|Default|GetDestination)) _newtrack_0) false false)
      (Utilities|FlowControl|Delay 5.0)
      (Transformation|SetActorLocation _returnvalue (Transformation|GetActorLocation) false false)
      (Utilities|FlowControl|Delay 0.2)
      (CallFunction|Loop))))

(fn ConstructionScript)