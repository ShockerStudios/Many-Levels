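; Pushable block that BP_Mover grabs and releases through Interact, attaching to the player while carried.
; Four side overlap triggers record the grab side and direction; grabbing snaps the player there, facing the block.
; Each toggle flips box collision, calls WallToggle with that direction on channel-matched BP_BlockWalls, and blends view between block and player.
; It also copies CameraThing into the player's CameraRotation, though that variable's setup logic is disconnected.
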(event OnComponentBeginOverlap(Left)
  (params (OverlappedComponent :type Primitive%20Component%20Object%20Reference) (OtherActor :type Actor%20Object%20Reference) (OtherComp :type Primitive%20Component%20Object%20Reference) (OtherBodyIndex :type Integer) (bFromSweep :type Boolean) (SweepResult :type Hit%20Result%20Structure%20%28by%20ref%29))
  (Utilities|Casting|CastToBP_Mover OtherActor)
  (Variables|Default|SetCurrentSide (Variables|Default|GetLeft))
  (Variables|Default|SetWallDirection 3))

(event OnComponentBeginOverlap(Right)
  (params (OverlappedComponent :type Primitive%20Component%20Object%20Reference) (OtherActor :type Actor%20Object%20Reference) (OtherComp :type Primitive%20Component%20Object%20Reference) (OtherBodyIndex :type Integer) (bFromSweep :type Boolean) (SweepResult :type Hit%20Result%20Structure%20%28by%20ref%29))
  (Utilities|Casting|CastToBP_Mover OtherActor)
  (Variables|Default|SetCurrentSide (Variables|Default|GetRight))
  (Variables|Default|SetWallDirection 1))

(event OnComponentBeginOverlap(UpCollision)
  (params (OverlappedComponent :type Primitive%20Component%20Object%20Reference) (OtherActor :type Actor%20Object%20Reference) (OtherComp :type Primitive%20Component%20Object%20Reference) (OtherBodyIndex :type Integer) (bFromSweep :type Boolean) (SweepResult :type Hit%20Result%20Structure%20%28by%20ref%29))
  (Utilities|Casting|CastToBP_Mover OtherActor)
  (Variables|Default|SetCurrentSide (Variables|Default|GetUpCollision))
  (Variables|Default|SetWallDirection 0))

(event OnComponentBeginOverlap(DownCollision)
  (params (OverlappedComponent :type Primitive%20Component%20Object%20Reference) (OtherActor :type Actor%20Object%20Reference) (OtherComp :type Primitive%20Component%20Object%20Reference) (OtherBodyIndex :type Integer) (bFromSweep :type Boolean) (SweepResult :type Hit%20Result%20Structure%20%28by%20ref%29))
  (Utilities|Casting|CastToBP_Mover OtherActor)
  (Variables|Default|SetCurrentSide (Variables|Default|GetDownCollision))
  (Variables|Default|SetWallDirection 2))

(event EventBeginPlay
  ;[1 1 1] Get Walls
  (bind _outactors (Actor|GetAllActorsOfClass "/Game/Sapphire/Cameron/Blueprints/BP_BlockWall.BP_BlockWall_C"))
  (for _array_element _outactors
    (if (== (Variables|/Game/Sapphire/Cameron/Blueprints/BP_BlockWall.BP_BlockWall_C|GetChannel _array_element) (Variables|Default|GetWall%20Channel))
      (Utilities|Array|Add (Variables|Default|GetMatching%20Walls) _array_element))))

(event EventInteract
  (bind _returnvalue (Game|GetPlayerController 0))
  (bind _box (Variables|Default|GetBox))
  (bind _asbp_mover (Utilities|Casting|CastToBP_Mover (Game|GetPlayerCharacter 0)))
  (bind _output_get (Variables|Default|SetPossesion _asbp_mover))
  (Variables|/Game/Sapphire/PossessableCharacters/Blueprints/BP_Mover.BP_Mover_C|SetCameraRotation _output_get (Variables|Default|GetCamera%20Thing))
  (if (Variables|/Game/Sapphire/PossessableCharacters/Blueprints/BP_Mover.BP_Mover_C|GetMovingCube _output_get)
    (Variables|/Game/Sapphire/PossessableCharacters/Blueprints/BP_Mover.BP_Mover_C|SetMovingCube (Variables|Default|GetPossesion) false)
    ;[1 1 1] Deactivate
    (Collision|SetCollisionEnabled _box "QueryAndPhysics")
    (for _array_element (Variables|Default|GetMatching%20Walls)
      (bind _asbp_block_wall (Utilities|Casting|CastToBP_BlockWall _array_element))
      (Default|WallToggle _asbp_block_wall (Variables|Default|GetWallDirection)))
    (Transformation|DetachFromActor "KeepWorld" "KeepWorld" "KeepWorld")
    (Game|Player|SetViewTargetwithBlend _returnvalue (Variables|Default|GetPossesion) 0.0 "VTBlend_Linear" 0.0 false)
    (else
      (Variables|/Game/Sapphire/PossessableCharacters/Blueprints/BP_Mover.BP_Mover_C|SetMovingCube (Variables|Default|GetPossesion) true)
      ;[1 1 1] Activate
      (Transformation|SetActorLocation (Variables|Default|GetPossesion) (Transformation|GetWorldLocation (Variables|Default|GetCurrentSide)) false false)
      (Transformation|SetActorRotation (Variables|Default|GetPossesion) (Math|Rotator|MakeRotator 0.0 0.0 (.yaw (Math|Rotator|FindLookatRotation (Transformation|GetActorLocation (Variables|Default|GetPossesion)) (Transformation|GetActorLocation)))))
      (Collision|SetCollisionEnabled _box "NoCollision")
      (for _array_element_2 (Variables|Default|GetMatching%20Walls)
        (bind _asbp_block_wall_2 (Utilities|Casting|CastToBP_BlockWall _array_element_2))
        (Default|WallToggle _asbp_block_wall_2 (Variables|Default|GetWallDirection)))
      (Transformation|AttachActorToActor (Variables|Default|GetPossesion) "None" "KeepWorld" "KeepWorld" "KeepWorld" true)
      (Game|Player|SetViewTargetwithBlend _returnvalue self 0.0 "VTBlend_Linear" 0.0 false))))

(fn ConstructionScript)