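; BP_Breakable_Villian is a breakable villain object whose destruction also opens a fake wall in the level.
; Its Destroy event hides the static and skeletal meshes and disables their collision instead of removing the actor.
; It then finds a BP_FakeWall through GetActorOfClass, hides that actor's root component without propagating to children, and disables the Wall component's collision.
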(event EventDestroy
  (bind _staticmesh (Variables|Default|GetStaticMesh))
  (bind _skeletalmesh (Variables|Default|GetSkeletalMesh))
  (Rendering|SetVisibility _staticmesh false false)
  (Collision|SetCollisionEnabled _staticmesh "NoCollision")
  (Rendering|SetVisibility _skeletalmesh false false)
  (Collision|SetCollisionEnabled _skeletalmesh "NoCollision")
  (bind _returnvalue (Actor|GetActorOfClass "/Game/Sapphire/Cameron/Blueprints/BP_FakeWall.BP_FakeWall_C"))
  (Rendering|SetVisibility (Variables|/Script/Engine.Actor|GetRootComponent _returnvalue) false false)
  (Collision|SetCollisionEnabled (Variables|/Game/Sapphire/Cameron/Blueprints/BP_FakeWall.BP_FakeWall_C|GetWall _returnvalue) "NoCollision"))

(fn ConstructionScript
  (|CallParentFunction))