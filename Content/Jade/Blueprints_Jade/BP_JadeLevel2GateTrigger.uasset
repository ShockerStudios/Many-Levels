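; BP_JadeLevel2GateTrigger is a one-shot trigger that shifts the Jade Level 2 gates when BP_Devvy overlaps it.
; It plays the gate-close sound at its SoundReferencePoint, then loops over every BP_JadeLevel2Gate in the world.
; Gates tagged "Exit" move up and all others move down by the same fixed offset, snapping instantly through root-component transforms with no animation.
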(event Collision|EventActorBeginOverlap
  (params (OtherActor :type Actor%20Object%20Reference))
  (Utilities|Casting|CastToBP_Devvy OtherActor)
  (Utilities|FlowControl|DoOnce false
    (:Completed
      (Audio|PlaySoundatLocation "/Game/Jade/Sounds_Jade/SoundCues_Jade/SC_GateCloseLevel2.SC_GateCloseLevel2" (Transformation|GetWorldLocation (Variables|Default|GetSoundReferencePoint)) "0, 0, 0" 1.0 1.0 0.0 0 0 0 0)
      (bind _outactors (Actor|GetAllActorsOfClass "/Game/Jade/Blueprints_Jade/BP_JadeLevel2Gate.BP_JadeLevel2Gate_C"))
      (for _array_element _outactors
        (if (Actor|ActorHasTag _array_element "Exit")
          (Transformation|SetRelativeTransform (Variables|/Script/Engine.Actor|GetRootComponent _array_element) (Math|Transform|MakeTransform (Math|Vector|MakeVector (.x (.location (Transformation|GetActorTransform _array_element))) (.y (.location (Transformation|GetActorTransform _array_element))) (+ (.z (.location (Transformation|GetActorTransform _array_element))) 3.5e+02)) (.rotation (Transformation|GetActorTransform _array_element)) (.scale (Transformation|GetActorTransform _array_element))) false false)
          (else
            (Transformation|SetRelativeTransform (Variables|/Script/Engine.Actor|GetRootComponent _array_element) (Math|Transform|MakeTransform (Math|Vector|MakeVector (.x (.location (Transformation|GetActorTransform _array_element))) (.y (.location (Transformation|GetActorTransform _array_element))) (- (.z (.location (Transformation|GetActorTransform _array_element))) 3.5e+02)) (.rotation (Transformation|GetActorTransform _array_element)) (.scale (Transformation|GetActorTransform _array_element))) false false)))))))

(fn ConstructionScript)