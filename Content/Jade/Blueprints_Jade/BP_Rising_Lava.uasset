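; Rising lava hazard that climbs through the level and kills the BP_Devvy character on contact.
; On BeginPlay it caches the Pos1 and Pos2 world locations, then a timeline with a variable play rate lerps the Lava component between them.
; Overlapping KillVolume destroys BP_Devvy and, after a short delay, opens the hard-coded 5Bryce level.
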(event OnComponentBeginOverlap(KillVolume)
  (params (OverlappedComponent :type Primitive%20Component%20Object%20Reference) (OtherActor :type Actor%20Object%20Reference) (OtherComp :type Primitive%20Component%20Object%20Reference) (OtherBodyIndex :type Integer) (bFromSweep :type Boolean) (SweepResult :type Hit%20Result%20Structure%20%28by%20ref%29))
  (bind _asbp_devvy (Utilities|Casting|CastToBP_Devvy OtherActor))
  (Actor|DestroyActor _asbp_devvy)
  (Utilities|FlowControl|Delay 2.0)
  (Game|OpenLevel(byName) "5Bryce"))

(event EventBeginPlay
  (|PositionInfo)
  (Components|Timeline|SetPlayRate (Variables|Default|GetRisingLava) (Variables|Default|GetPlayrate))
  (bind _newtrack_0 (Timeline|RisingLava Play)
    (:Update
      (Transformation|SetWorldLocation (Variables|Default|GetLava) (Math|Vector|Lerp(Vector) (Variables|Default|GetPosition1) (Variables|Default|GetPosition2) _newtrack_0) false false))))

(fn ConstructionScript)