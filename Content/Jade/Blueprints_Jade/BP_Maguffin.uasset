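; BP_Maguffin is an actor that shows a text prompt when the player character BP_Devvy overlaps it while not holding an object.
; The text hides when the overlap ends, or when an overlap begins while Devvy is already holding something.
; Every tick, its Scene component rotates toward the player camera, using a look-at rotation applied as a relative rotation.
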(event EventTick
  (params (DeltaSeconds :type Float%20%28single-precision%29))
  (bind _scene (Variables|Default|GetScene))
  (Transformation|SetRelativeRotation _scene (Math|Rotator|FindLookatRotation (Transformation|GetWorldLocation _scene) (Camera|GetCameraLocation (Game|GetPlayerCameraManager 0))) false false))

(event Collision|EventActorBeginOverlap
  (params (OtherActor :type Actor%20Object%20Reference))
  (bind _textrender (Variables|Default|GetTextRender))
  (if (not (Variables|/Game/Blueprints/BP_Devvy.BP_Devvy_C|GetHolding%20object (.AsBP%20Devvy (Utilities|Casting|CastToBP_Devvy (Game|GetPlayerCharacter 0)))))
    (Utilities|Casting|CastToBP_Devvy OtherActor)
    (Rendering|SetVisibility _textrender true false)
    (else
      (Rendering|SetVisibility _textrender false false))))

(event Collision|EventActorEndOverlap
  (params (OtherActor :type Actor%20Object%20Reference))
  (Rendering|SetVisibility (Variables|Default|GetTextRender) false false))

(fn ConstructionScript)