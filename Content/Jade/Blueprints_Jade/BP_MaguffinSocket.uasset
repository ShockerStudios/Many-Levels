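; BP_MaguffinSocket is a puzzle socket that opens a castle iron gate when a BP_Maguffin enters its trigger box.
; On overlap it destroys the maguffin, shows the sword holder mesh, hides the gate and disables its collision, marks itself solved and clears HoldingObject on the player's BP_Devvy.
; Until solved, any other overlapping actor reveals a text prompt, which hides again when an overlap ends.
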(event OnComponentBeginOverlap(Box)
  (params (OverlappedComponent :type Primitive%20Component%20Object%20Reference) (OtherActor :type Actor%20Object%20Reference) (OtherComp :type Primitive%20Component%20Object%20Reference) (OtherBodyIndex :type Integer) (bFromSweep :type Boolean) (SweepResult :type Hit%20Result%20Structure%20%28by%20ref%29))
  (bind _sm_bld_castle_iron_gate_01 (Variables|Default|GetSM_Bld_Castle_Iron_Gate_01))
  (Utilities|Casting|CastToBP_Maguffin OtherActor
    (:then
      (bind _asbp_devvy (Utilities|Casting|CastToBP_Devvy (Game|GetPlayerCharacter 0)))
      (Rendering|SetVisibility (Variables|Default|GetSM_Item_SwordHolder) true true)
      (Actor|DestroyActor OtherActor)
      (Rendering|SetVisibility _sm_bld_castle_iron_gate_01 false false)
      (Collision|SetCollisionEnabled _sm_bld_castle_iron_gate_01 "NoCollision")
      (Rendering|SetVisibility (Variables|Default|GetTextRender) false false)
      (Variables|Default|SetSolved true)
      (Variables|/Game/Blueprints/BP_Devvy.BP_Devvy_C|SetHolding%20object _asbp_devvy false))
    (:CastFailed
      (if (not (Variables|Default|GetSolved))
        (Rendering|SetVisibility (Variables|Default|GetTextRender) true false)))))

(event OnComponentEndOverlap(Box)
  (params (OverlappedComponent :type Primitive%20Component%20Object%20Reference) (OtherActor :type Actor%20Object%20Reference) (OtherComp :type Primitive%20Component%20Object%20Reference) (OtherBodyIndex :type Integer))
  (Rendering|SetVisibility (Variables|Default|GetTextRender) false false))

(event EventBeginPlay
  (Rendering|SetVisibility (Variables|Default|GetTextRender) false false))

(fn ConstructionScript)