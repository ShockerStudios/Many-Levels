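; BP_Level2Tutorial is a world text prompt for the Level 2 tutorial that vanishes once the player wall runs near it.
; Each tick it sets the text from a string variable and line traces from its root to the BP_Devvy player against pawns.
; If the hit distance is under a threshold while the player is in a wall run, it hides the text, with no logic to show it again.
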(event EventTick
  (params (DeltaSeconds :type Float%20%28single-precision%29))
  (Rendering|Components|TextRender|SetText (Variables|Default|GetTextRender) (Utilities|Text|ToText(String) (Variables|Default|GetTextString)))
  (bind _asbp_devvy (Utilities|Casting|CastToBP_Devvy (Game|GetPlayerCharacter 0)))
  (bind _outhit (Collision|LineTraceForObjects (Transformation|GetWorldLocation (Variables|Default|GetDefaultSceneRoot)) (Transformation|GetActorLocation _asbp_devvy) (Utilities|Array|MakeArray "ObjectTypeQuery3") false 0 "None"))
  (if (< (.distance _outhit) (Variables|Default|GetDistanceNeededToVanish))
    (if (Variables|/Game/Blueprints/BP_Devvy.BP_Devvy_C|GetbInWallRun _asbp_devvy)
      (Rendering|SetVisibility (Variables|Default|GetTextRender) false false))))

(fn ConstructionScript)