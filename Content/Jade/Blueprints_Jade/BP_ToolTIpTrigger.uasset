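; BP_ToolTIpTrigger is a trigger actor that shows a tooltip on the player's UI when BP_Devvy overlaps it.
; Overlap copies VolumeText into the character's ToolTipToDisplay and enters a DoOnce that plays the UI's ToolTipAnimation.
; After a fixed delay it flags the display as finished, and Tick then resets the DoOnce so the tooltip can show again.
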(event Collision|EventActorBeginOverlap
  (params (OtherActor :type Actor%20Object%20Reference))
  (bind _asbp_devvy (Utilities|Casting|CastToBP_Devvy OtherActor))
  (Variables|Default|SetbPlayerIsInVolume true)
  (Variables|/Game/Blueprints/BP_Devvy.BP_Devvy_C|SetToolTipToDisplay _asbp_devvy (Variables|Default|GetVolumeText))
  (Utilities|FlowControl|DoOnce false
    (:Completed
      (UserInterface|Animation|PlayAnimation (Variables|/Game/Blueprints/BP_Devvy.BP_Devvy_C|GetPlayerUI _asbp_devvy) (Variables|/Game/Jade/Blueprints_Jade/BP_PlayerUI_Jade.BP_PlayerUI_Jade_C|GetToolTipAnimation (Variables|/Game/Blueprints/BP_Devvy.BP_Devvy_C|GetPlayerUI _asbp_devvy)) 0.0 1 "Forward" 1.0 false)
      (Utilities|FlowControl|Delay 6.5)
      (Variables|Default|SetbPlayerIsInVolume false)
      (Variables|Default|SetbIsDoneDisplaying true))))

(event EventTick
  (params (DeltaSeconds :type Float%20%28single-precision%29))
  (bind _output_get (Variables|Default|SetbPlayerIsInVolume false))
  (if (and (not _output_get) (Variables|Default|GetbIsDoneDisplaying))
    (Variables|Default|SetbIsDoneDisplaying false)
    (Utilities|FlowControl|DoOnce false) ; enters at Reset
  ))

(fn ConstructionScript)