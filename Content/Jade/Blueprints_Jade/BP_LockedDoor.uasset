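; BP_LockedDoor is a locked door that opens when a BP_Key actor enters its trigger box.
; The key overlap hides the door mesh and text, disables door collision, marks it solved, plays a sound, clears BP_Devvy's HoldingObject flag and destroys the key.
; Other overlaps show the text until the door is solved, and any end overlap hides it.
; Tick turns the Scene component toward the player camera, billboard-style.
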(event OnComponentBeginOverlap(Box)
  (params (OverlappedComponent :type Primitive%20Component%20Object%20Reference) (OtherActor :type Actor%20Object%20Reference) (OtherComp :type Primitive%20Component%20Object%20Reference) (OtherBodyIndex :type Integer) (bFromSweep :type Boolean) (SweepResult :type Hit%20Result%20Structure%20%28by%20ref%29))
  (bind _asbp_key (Utilities|Casting|CastToBP_Key OtherActor)
    (:then
      (Rendering|SetVisibility (Variables|Default|GetSM_Bld_Castle_Door_R) false true)
      (Collision|SetCollisionEnabled (Variables|Default|GetDoorColision) "NoCollision")
      (Variables|Default|SetSolved true)
      (Variables|/Game/Blueprints/BP_Devvy.BP_Devvy_C|SetHolding%20object (.AsBP%20Devvy (Utilities|Casting|CastToBP_Devvy (Game|Player|GetPlayerPawn 0))) false)
      (Audio|PlaySound2D "/Game/Jade/Sounds_Jade/CAFOFO_RPGSounds/Doors_Lockers/Door_7_1_Open.Door_7_1_Open" 1.0 1.0 0.0 0 0)
      (Actor|DestroyActor OtherActor))
    (:CastFailed
      (if (not (Variables|Default|GetSolved))
        (Rendering|SetVisibility (Variables|Default|GetTextRender) true false)))))

(event OnComponentEndOverlap(Box)
  (params (OverlappedComponent :type Primitive%20Component%20Object%20Reference) (OtherActor :type Actor%20Object%20Reference) (OtherComp :type Primitive%20Component%20Object%20Reference) (OtherBodyIndex :type Integer))
  (Rendering|SetVisibility (Variables|Default|GetTextRender) false false))

(event EventTick
  (params (DeltaSeconds :type Float%20%28single-precision%29))
  (bind _scene (Variables|Default|GetScene))
  (Transformation|SetRelativeRotation _scene (Math|Rotator|FindLookatRotation (Transformation|GetWorldLocation _scene) (Camera|GetCameraLocation (Game|GetPlayerCameraManager 0))) false false))

(fn ConstructionScript)