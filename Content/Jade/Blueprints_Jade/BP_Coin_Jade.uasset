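; BP_Coin_Jade is a collectible coin that floats, spins and awards score to the player.
; On BeginPlay, one timeline lerps the root between its start location and a point slightly above it.
; A second timeline adds yaw to the starting rotation and restarts whenever it finishes.
; On overlap with BP_Devvy, the coin adds InstScoreValue to that actor's Score and destroys itself.
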(event EventBeginPlay
  ;[1 1 1] Allows Coin to float up and down while spinning
  (Utilities|FlowControl|Sequence
    (:then_0
      (bind _output_get (Variables|Default|SetCoinLocation (Transformation|GetActorLocation)))
      (bind _makeobjectfloat (Timeline|SetTransformInterpolation Play)
        (:Update
          (Transformation|SetRelativeTransform (Variables|Default|GetDefaultSceneRoot) (Math|Transform|MakeTransform (Math|Vector|Lerp(Vector) _output_get (+ _output_get "0,0,20.000000") _makeobjectfloat) "0, 0, 0" "1.000000,1.000000,1.000000") false false))))
    (:then_1
      ;;[1 1 1] RotateCoin
      (Variables|Default|SetCoinStartRotation (Transformation|GetActorRotation))
      (bind _rotateobject (Timeline|RotateCoin Play)
        (:Update
          (Transformation|SetRelativeRotation (Variables|Default|GetDefaultSceneRoot) (Math|Rotator|MakeRotator (.roll (Variables|Default|GetCoinStartRotation)) (.pitch (Variables|Default|GetCoinStartRotation)) (+ (.yaw (Variables|Default|GetCoinStartRotation)) _rotateobject)) false false))
        (:Finished
          (Timeline|RotateCoin PlayFromStart))))))

(event Collision|EventActorBeginOverlap
  (params (OtherActor :type Actor%20Object%20Reference))
  ;[1 1 1] Add Score to Player
  (bind _asbp_devvy (Utilities|Casting|CastToBP_Devvy OtherActor))
  (Variables|/Game/Blueprints/BP_Devvy.BP_Devvy_C|SetScore _asbp_devvy (+ (Variables|/Game/Blueprints/BP_Devvy.BP_Devvy_C|GetScore _asbp_devvy) (Variables|Default|GetInstScoreValue)))
  (Actor|DestroyActor))

(fn ConstructionScript)