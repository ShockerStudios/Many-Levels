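; BP_Torch is a torch actor that shows a text prompt when the BP_Devvy character comes near.
; Each Tick it rotates a scene component to face the player camera.
; On actor overlap it shows the TextRender only if BP_Devvy is not holding an object, and the box's end overlap hides it again.
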(event OnComponentEndOverlap(Box)
  (params (OverlappedComponent :type Primitive%20Component%20Object%20Reference) (OtherActor :type Actor%20Object%20Reference) (OtherComp :type Primitive%20Component%20Object%20Reference) (OtherBodyIndex :type Integer))
  (Rendering|SetVisibility (Variables|Default|GetTextRender) false false))

(event Collision|EventActorBeginOverlap
  (params (OtherActor :type Actor%20Object%20Reference))
  (bind _textrender (Variables|Default|GetTextRender))
  (bind _asbp_devvy (Utilities|Casting|CastToBP_Devvy OtherActor))
  (if (not (Variables|/Game/Blueprints/BP_Devvy.BP_Devvy_C|GetHolding%20object _asbp_devvy))
    (Rendering|SetVisibility _textrender true false)
    (else
      (Rendering|SetVisibility _textrender false false))))

(event EventTick
  (params (DeltaSeconds :type Float%20%28single-precision%29))
  (bind _scene (Variables|Default|GetScene))
  ;[1 1 1] Look At Camera
  (Transformation|SetRelativeRotation _scene (Math|Rotator|FindLookatRotation (Transformation|GetWorldLocation _scene) (Camera|GetCameraLocation (Game|GetPlayerCameraManager 0))) false false))

(fn ConstructionScript)